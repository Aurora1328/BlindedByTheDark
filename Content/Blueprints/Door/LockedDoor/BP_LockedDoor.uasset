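; BP_LockedDoor is an interactable door that stays shut until unlocked by a key or a bound UnlockDoor event targeting it.
; Interact on a locked door spends one of the player's held keys, first matching and removing a key ID if required, then opens it.
; Unlocked doors toggle via timelines rotating the hinge, with sounds and DoOnce guards against retriggering.
; Optional UseDOT gates toggling on a rounded door-to-player orientation dot product.
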(event Custom|UnlockDoorEvent
  (EventDispatchers|BindEventtoUnlockDoor (delegate Custom|UnlockDoorBind)))

(event Custom|UnlockDoorBind
  (params (DoorToUnlock :type Actor%20Object%20Reference))
  (if (== DoorToUnlock self)
    (Variables|Default|SetDoorUnlocked? true)))

(event EventBeginPlay
  (|CallParentFunction)
  (CallFunction|UnlockDoorEvent))

(event Collision|EventActorBeginOverlap
  (params (OtherActor :type Actor%20Object%20Reference))
  (|CallParentFunction OtherActor) ; This node is disabled and will not be called.\nDrag off pins to build functionality.
)

(event EventTick
  (params (DeltaSeconds :type Float%20%28single-precision%29))
  (|CallParentFunction DeltaSeconds) ; This node is disabled and will not be called.\nDrag off pins to build functionality.
)

(event EventInteract
  (params (Character :type BP%20First%20Person%20Character%20Object%20Reference))
  (bind _playerref (Variables|Default|GetPlayerRef))
  (switch Utilities|FlowControl|Switch|SwitchonE_DoorType (.DoorType (Utilities|Struct|BreakS_DoorInfo (.DoorInfo (Utilities|Struct|BreakS_ItemInfo (Variables|Default|GetItemInfo)))))
    (:NewEnumerator2
      (if (Variables|Default|GetDoorUnlocked?)
        (if (Variables|Default|GetUseDOT?) :!label _label
          (bind _output_get (Variables|Default|SetDirection (Math|Float|Round (Math|Vector|DotProduct (Math|Vector|GetForwardVector (Transformation|GetActorRotation)) (Math|Vector|GetRightVector (Transformation|GetActorRotation (Game|GetPlayerCharacter 0)))))))
          (if (not (== _output_get 0))
            (if (Variables|Default|GetDoorOpen?)
              (Utilities|FlowControl|DoOnce false :!label _label_2
                (:Completed
                  (Audio|PlaySound2D "/Engine/VREditor/Sounds/UI/Click_on_Button.Click_on_Button" 1.0 1.0 0.0 0 0)
                  (bind _doorangle (Timeline|Timeline_1 PlayFromStart)
                    (:Update
                      (Transformation|SetRelativeRotation (Variables|Default|GetHinge) (Math|Rotator|MakeRotator 0.0 0.0 _doorangle) false false))
                    (:Finished
                      (Variables|Default|SetDoorOpen? false)
                      (goto _label_2 Reset)))))
              (else
                (Utilities|FlowControl|DoOnce false :!label _label_3
                  (:Completed
                    (Audio|PlaySound2D "/Engine/VREditor/Sounds/UI/Click_on_Button_Cue.Click_on_Button_Cue" 1.0 1.0 0.0 0 0)
                    (bind _doorangle_2 (Timeline|Timeline_0 PlayFromStart)
                      (:Update
                        (Transformation|SetRelativeRotation (Variables|Default|GetHinge) (Math|Rotator|MakeRotator 0.0 0.0 _doorangle_2) false false))
                      (:Finished
                        (Variables|Default|SetDoorOpen? true)
                        (goto _label_3 Reset))))))))
          (elif (Variables|Default|GetDoorOpen?)
            (Utilities|FlowControl|DoOnce false :!label _label_4
              (:Completed
                (Audio|PlaySound2D "/Engine/VREditor/Sounds/UI/Click_on_Button.Click_on_Button" 1.0 1.0 0.0 0 0)
                (bind _doorangle_3 (Timeline|Timeline PlayFromStart)
                  (:Update
                    (Transformation|SetRelativeRotation (Variables|Default|GetHinge) (Math|Rotator|MakeRotator 0.0 0.0 _doorangle_3) false false))
                  (:Finished
                    (Variables|Default|SetDoorOpen? false)
                    (goto _label_4 Reset)))))
            (else
              (Utilities|FlowControl|DoOnce false :!label _label_5
                (:Completed
                  (Audio|PlaySound2D "/Engine/VREditor/Sounds/UI/Click_on_Button_Cue.Click_on_Button_Cue" 1.0 1.0 0.0 0 0)
                  (bind _doorangle_4 (Timeline|DoorOpen PlayFromStart)
                    (:Update
                      (Transformation|SetRelativeRotation (Variables|Default|GetHinge) (Math|Rotator|MakeRotator 0.0 0.0 _doorangle_4) false false))
                    (:Finished
                      (Variables|Default|SetDoorOpen? true)
                      (goto _label_5 Reset))))))))
        (elif (Variables|Default|GetIsIDRequired?)
          (bind _array_element (Utilities|Array|ForEachLoopwithBreak (Variables|/Game/FirstPerson/Blueprints/BP_FirstPersonCharacter.BP_FirstPersonCharacter_C|GetKeyID'sHeld (Variables|Default|GetPlayerRef)) :!label _label_6)
            (:LoopBody
              (if (== _array_element (Variables|Default|GetIDRequired))
                (Variables|Default|SetIDFound? true)
                (goto _label_6 Break)))
            (:Completed
              (if (Variables|Default|GetIDFound?)
                (Utilities|Array|RemoveItem (Variables|/Game/FirstPerson/Blueprints/BP_FirstPersonCharacter.BP_FirstPersonCharacter_C|GetKeyID'sHeld (Variables|Default|GetPlayerRef)) (Variables|Default|GetIDRequired))
                (if (> (Variables|/Game/FirstPerson/Blueprints/BP_FirstPersonCharacter.BP_FirstPersonCharacter_C|GetKeysHeld (Variables|Default|GetPlayerRef)) 0) :!label _label_7
                  (Variables|/Game/FirstPerson/Blueprints/BP_FirstPersonCharacter.BP_FirstPersonCharacter_C|SetKeysHeld _playerref (Math|Integer|Clamp(Integer) (- (Variables|/Game/FirstPerson/Blueprints/BP_FirstPersonCharacter.BP_FirstPersonCharacter_C|GetKeysHeld _playerref) 1) 0 99))
                  (Default|CallUpdateKeysHeld (Variables|Default|GetPlayerRef))
                  (Variables|Default|SetDoorUnlocked? true)
                  (goto _label)))))
          (else
            (goto _label_7)))))))

(fn ConstructionScript
  (|CallParentFunction))