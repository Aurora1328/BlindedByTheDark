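; BP_Planks is a three-plank obstacle that the player can knock loose once scrap has been collected.
; BeginPlay freezes the planks with collision on and caches a BP_Scrap actor from the level; a Box overlap toggles player input.
; On IA_Interact, if that scrap's IsCollectedScrap is true, the planks simulate physics and ignore Pawn collision.
; The HasPlayedSound check skips the Scrap sound on first interaction and plays it on later ones.
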(event OnComponentBeginOverlap(Box)
  (params (OverlappedComponent :type Primitive%20Component%20Object%20Reference) (OtherActor :type Actor%20Object%20Reference) (OtherComp :type Primitive%20Component%20Object%20Reference) (OtherBodyIndex :type Integer) (bFromSweep :type Boolean) (SweepResult :type Hit%20Result%20Structure%20%28by%20ref%29))
  (Input|EnableInput (Game|GetPlayerController 0)))

(event OnComponentEndOverlap(Box)
  (params (OverlappedComponent :type Primitive%20Component%20Object%20Reference) (OtherActor :type Actor%20Object%20Reference) (OtherComp :type Primitive%20Component%20Object%20Reference) (OtherBodyIndex :type Integer))
  (Input|DisableInput (Game|GetPlayerController 0)))

(event Input|EnhancedActionEvents|EnhancedInputActionIA_Interact
  (params (ActionValue :type Boolean) (ElapsedSeconds :type Float%20%28double-precision%29) (TriggeredSeconds :type Float%20%28double-precision%29) (InputAction :type Input%20Action%20Object%20Reference :default "/Game/FirstPerson/Input/Actions/IA_Interact.IA_Interact"))
  (if (Variables|/Game/Blueprints/Door/BP_Scrap.BP_Scrap_C|GetIsCollectedScrap? (stale EventBeginPlay _asbp_scrap))
    (Utilities|FlowControl|Sequence
      (:then_0
        (Physics|SetSimulatePhysics (Variables|Default|GetStatic%20Mesh) true)
        (Collision|SetCollisionResponsetoChannel (Variables|Default|GetStatic%20Mesh) "ECC_Pawn" "ECR_Ignore")
        (if (Variables|Default|GetHasPlayedSound)
          (Audio|PlaySound2D "/Game/Audio/Sounds/scrap.scrap" 1.0 1.0 0.0 0 0)
          (else
            (Variables|Default|SetHasPlayedSound true))))
      (:then_1
        (Physics|SetSimulatePhysics (Variables|Default|GetStatic%20Mesh1) true)
        (Collision|SetCollisionResponsetoChannel (Variables|Default|GetStatic%20Mesh1) "ECC_Pawn" "ECR_Ignore"))
      (:then_2
        (Physics|SetSimulatePhysics (Variables|Default|GetStatic%20Mesh2) true)
        (Collision|SetCollisionResponsetoChannel (Variables|Default|GetStatic%20Mesh2) "ECC_Pawn" "ECR_Ignore")))))

(event EventBeginPlay
  (Utilities|FlowControl|Sequence
    (:then_0
      (Collision|SetCollisionEnabled (Variables|Default|GetStatic%20Mesh) "QueryAndPhysics")
      (Physics|SetSimulatePhysics (Variables|Default|GetStatic%20Mesh) false))
    (:then_1
      (Collision|SetCollisionEnabled (Variables|Default|GetStatic%20Mesh1) "QueryAndPhysics")
      (Physics|SetSimulatePhysics (Variables|Default|GetStatic%20Mesh1) false))
    (:then_2
      (Collision|SetCollisionEnabled (Variables|Default|GetStatic%20Mesh2) "QueryAndPhysics")
      (Physics|SetSimulatePhysics (Variables|Default|GetStatic%20Mesh2) false))
    (:then_3
      (bind _outactors (Actor|GetAllActorsOfClass "/Game/Blueprints/Door/BP_Scrap.BP_Scrap_C"))
      (for _array_element _outactors
        (bind _asbp_scrap (Utilities|Casting|CastToBP_Scrap _array_element))))))

(fn ConstructionScript)