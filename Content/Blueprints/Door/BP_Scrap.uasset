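; BP_Scrap is a collectible scrap pickup that the player gathers with the interact input.
; Its box overlap enables and disables player input on the actor, so IA_Interact only fires while something overlaps it.
; Interacting marks the scrap collected, hides the mesh, turns off its collision and tells the first-person character's HUD to show the scrap icon.
; The construction script applies the configurable ItemMesh to the static mesh.
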(event OnComponentBeginOverlap(Box)
  (params (OverlappedComponent :type Primitive%20Component%20Object%20Reference) (OtherActor :type Actor%20Object%20Reference) (OtherComp :type Primitive%20Component%20Object%20Reference) (OtherBodyIndex :type Integer) (bFromSweep :type Boolean) (SweepResult :type Hit%20Result%20Structure%20%28by%20ref%29))
  (Input|EnableInput (Game|GetPlayerController 0)))

(event OnComponentEndOverlap(Box)
  (params (OverlappedComponent :type Primitive%20Component%20Object%20Reference) (OtherActor :type Actor%20Object%20Reference) (OtherComp :type Primitive%20Component%20Object%20Reference) (OtherBodyIndex :type Integer))
  (Input|DisableInput (Game|GetPlayerController 0)))

(event Input|EnhancedActionEvents|EnhancedInputActionIA_Interact
  (params (ActionValue :type Boolean) (ElapsedSeconds :type Float%20%28double-precision%29) (TriggeredSeconds :type Float%20%28double-precision%29) (InputAction :type Input%20Action%20Object%20Reference :default "/Game/FirstPerson/Input/Actions/IA_Interact.IA_Interact"))
  (Variables|Default|SetIsCollectedScrap? true)
  (Rendering|SetVisibility (Variables|Default|GetStatic%20Mesh) false false)
  (Collision|SetCollisionEnabled (Variables|Default|GetStatic%20Mesh) "NoCollision")
  (bind _asbp_first_person_character (Utilities|Casting|CastToBP_FirstPersonCharacter (Pawn|GetControlledPawn (Game|GetPlayerController 0))))
  (Default|ShowScrapIcon (Variables|/Game/FirstPerson/Blueprints/BP_FirstPersonCharacter.BP_FirstPersonCharacter_C|GetHUDRef _asbp_first_person_character)))

(fn ConstructionScript
  (Utilities|FlowControl|Sequence
    (:then_0
      (Components|StaticMesh|SetStaticMesh (Variables|Default|GetStatic%20Mesh) (Variables|Default|GetItem%20Mesh)))))