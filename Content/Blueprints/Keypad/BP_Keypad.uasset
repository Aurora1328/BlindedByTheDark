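; BP_Keypad is an interactable four-digit keypad that unlocks a door when the correct code is entered.
; Interact uses a FlipFlop, debounced by DoOnce and Delay, to blend the view to the keypad, freezing movement and showing the cursor, or back.
; Clickable digit components feed UpdateKeypadCode, which updates the screen widget and compares its input to CodeRequired.
; Success exits and calls BP_LockedDoor with DoorToUnlock; failure resets the entry.
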(event OnClicked(Button_0)
  (params (TouchedComponent :type Primitive%20Component%20Object%20Reference) (ButtonPressed :type Key%20Structure))
  ;[0.15 0.15 0.15 0.5] Enter Code
  (if (== ButtonPressed "LeftMouseButton")
    (Audio|PlaySound2D "/Engine/VREditor/Sounds/UI/Click_on_Button.Click_on_Button" 1.0 1.0 0.0 0 0)
    (Utilities|UpdateKeypadCode
      (:Success
        (Default|CallUnlockDoor (Variables|Default|GetLockedDoorRef) (Variables|Default|GetDoorToUnlock))))))

(event OnClicked(Button_1)
  (params (TouchedComponent :type Primitive%20Component%20Object%20Reference) (ButtonPressed :type Key%20Structure))
  ;[0.15 0.15 0.15 0.5] Enter Code
  (if (== ButtonPressed "LeftMouseButton")
    (Audio|PlaySound2D "/Engine/VREditor/Sounds/UI/Click_on_Button.Click_on_Button" 1.0 1.0 0.0 0 0)
    (Utilities|UpdateKeypadCode 1
      (:Success
        (Default|CallUnlockDoor (Variables|Default|GetLockedDoorRef) (Variables|Default|GetDoorToUnlock))))))

(event OnClicked(Button_2)
  (params (TouchedComponent :type Primitive%20Component%20Object%20Reference) (ButtonPressed :type Key%20Structure))
  ;[0.15 0.15 0.15 0.5] Enter Code
  (if (== ButtonPressed "LeftMouseButton")
    (Audio|PlaySound2D "/Engine/VREditor/Sounds/UI/Click_on_Button.Click_on_Button" 1.0 1.0 0.0 0 0)
    (Utilities|UpdateKeypadCode 2
      (:Success
        (Default|CallUnlockDoor (Variables|Default|GetLockedDoorRef) (Variables|Default|GetDoorToUnlock))))))

(event OnClicked(Button_3)
  (params (TouchedComponent :type Primitive%20Component%20Object%20Reference) (ButtonPressed :type Key%20Structure))
  ;[0.15 0.15 0.15 0.5] Enter Code
  (if (== ButtonPressed "LeftMouseButton")
    (Audio|PlaySound2D "/Engine/VREditor/Sounds/UI/Click_on_Button.Click_on_Button" 1.0 1.0 0.0 0 0)
    (Utilities|UpdateKeypadCode 3
      (:Success
        (Default|CallUnlockDoor (Variables|Default|GetLockedDoorRef) (Variables|Default|GetDoorToUnlock))))))

(event OnClicked(Button_4)
  (params (TouchedComponent :type Primitive%20Component%20Object%20Reference) (ButtonPressed :type Key%20Structure))
  ;[0.15 0.15 0.15 0.5] Enter Code
  (if (== ButtonPressed "LeftMouseButton")
    (Audio|PlaySound2D "/Engine/VREditor/Sounds/UI/Click_on_Button.Click_on_Button" 1.0 1.0 0.0 0 0)
    (Utilities|UpdateKeypadCode 4
      (:Success
        (Default|CallUnlockDoor (Variables|Default|GetLockedDoorRef) (Variables|Default|GetDoorToUnlock))))))

(event OnClicked(Button_5)
  (params (TouchedComponent :type Primitive%20Component%20Object%20Reference) (ButtonPressed :type Key%20Structure))
  ;[0.15 0.15 0.15 0.5] Enter Code
  (if (== ButtonPressed "LeftMouseButton")
    (Audio|PlaySound2D "/Engine/VREditor/Sounds/UI/Click_on_Button.Click_on_Button" 1.0 1.0 0.0 0 0)
    (Utilities|UpdateKeypadCode 5
      (:Success
        (Default|CallUnlockDoor (Variables|Default|GetLockedDoorRef) (Variables|Default|GetDoorToUnlock))))))

(event OnClicked(Button_6)
  (params (TouchedComponent :type Primitive%20Component%20Object%20Reference) (ButtonPressed :type Key%20Structure))
  ;[0.15 0.15 0.15 0.5] Enter Code
  (if (== ButtonPressed "LeftMouseButton")
    (Audio|PlaySound2D "/Engine/VREditor/Sounds/UI/Click_on_Button.Click_on_Button" 1.0 1.0 0.0 0 0)
    (Utilities|UpdateKeypadCode 6
      (:Success
        (Default|CallUnlockDoor (Variables|Default|GetLockedDoorRef) (Variables|Default|GetDoorToUnlock))))))

(event OnClicked(Button_7)
  (params (TouchedComponent :type Primitive%20Component%20Object%20Reference) (ButtonPressed :type Key%20Structure))
  ;[0.15 0.15 0.15 0.5] Enter Code
  (if (== ButtonPressed "LeftMouseButton")
    (Audio|PlaySound2D "/Engine/VREditor/Sounds/UI/Click_on_Button.Click_on_Button" 1.0 1.0 0.0 0 0)
    (Utilities|UpdateKeypadCode 7
      (:Success
        (Default|CallUnlockDoor (Variables|Default|GetLockedDoorRef) (Variables|Default|GetDoorToUnlock))))))

(event OnClicked(Button_8)
  (params (TouchedComponent :type Primitive%20Component%20Object%20Reference) (ButtonPressed :type Key%20Structure))
  ;[0.15 0.15 0.15 0.5] Enter Code
  (if (== ButtonPressed "LeftMouseButton")
    (Audio|PlaySound2D "/Engine/VREditor/Sounds/UI/Click_on_Button.Click_on_Button" 1.0 1.0 0.0 0 0)
    (Utilities|UpdateKeypadCode 8
      (:Success
        (Default|CallUnlockDoor (Variables|Default|GetLockedDoorRef) (Variables|Default|GetDoorToUnlock))))))

(event OnClicked(Button_9)
  (params (TouchedComponent :type Primitive%20Component%20Object%20Reference) (ButtonPressed :type Key%20Structure))
  ;[0.15 0.15 0.15 0.5] Enter Code
  (if (== ButtonPressed "LeftMouseButton")
    (Audio|PlaySound2D "/Engine/VREditor/Sounds/UI/Click_on_Button.Click_on_Button" 1.0 1.0 0.0 0 0)
    (Utilities|UpdateKeypadCode 9
      (:Success
        (Default|CallUnlockDoor (Variables|Default|GetLockedDoorRef) (Variables|Default|GetDoorToUnlock))))))

(event EventBeginPlay
  ;[0.15 0.15 0.15 0.5] Event Begin Play
  (bind _asbp_first_person_character (Utilities|Casting|CastToBP_FirstPersonCharacter (Game|GetPlayerCharacter 0)))
  (Variables|Default|SetPlayerRef _asbp_first_person_character)
  (bind _aswbp_keypad_screen (Utilities|Casting|CastToWBP_KeypadScreen (UserInterface|GetWidget (Variables|Components|GetScreenNumbersWidget))))
  (Variables|Default|SetKeypadScreenRef _aswbp_keypad_screen)
  (bind _returnvalue (Actor|GetActorOfClass "/Game/Blueprints/Door/LockedDoor/BP_LockedDoor.BP_LockedDoor_C"))
  (Variables|Default|SetLockedDoorRef _returnvalue))

(event EventInteract
  (params (Character :type BP%20First%20Person%20Character%20Object%20Reference))
  (bind _returnvalue (Game|GetPlayerController 0))
  (bind _returnvalue_2 (Game|GetPlayerController 0))
  ;[0.15 0.15 0.15 0.5] Interaction
  (if (not (Variables|Default|GetdoorIsNotLocked?))
    (Utilities|FlowControl|DoOnce false :!label _label
      (:Completed
        (Utilities|FlowControl|FlipFlop
          (:A
            (Game|Player|SetViewTargetwithBlend (Game|GetPlayerController 0) self 0.3 "VTBlend_Linear" 0.0 false)
            (Widget|SetVisibility (Variables|/Game/FirstPerson/Widgets/WBP_HUD.WBP_HUD_C|GetCrosshairBorder (Variables|/Game/FirstPerson/Blueprints/BP_FirstPersonCharacter.BP_FirstPersonCharacter_C|GetHUDRef (Variables|Default|GetPlayerRef))) "Hidden")
            (Audio|PlaySound2D "/Engine/VREditor/Sounds/UI/Dockable_Window_Drop.Dockable_Window_Drop" 1.0 1.0 0.0 0 0)
            (Pawn|Components|CharacterMovement|SetMovementMode (Variables|/Script/Engine.Character|GetCharacterMovement (Variables|Default|GetPlayerRef)) "MOVE_None" 0)
            (Variables|/Script/Engine.PlayerController|SetbShowMouseCursor _returnvalue true)
            (Input|SetInputModeGameandUI _returnvalue 0 "DoNotLock" true false)
            (Class|BPIKeypad|SetCurrentKeypad(Message) (UserInterface|GetWidget (Variables|Components|GetScreenNumbersWidget)) self)
            (Utilities|FlowControl|Delay 0.3))
          (:B
            (Game|Player|SetViewTargetwithBlend (Game|GetPlayerController 0) (Variables|Default|GetPlayerRef) 0.3 "VTBlend_Linear" 0.0 false)
            (Widget|SetVisibility (Variables|/Game/FirstPerson/Widgets/WBP_HUD.WBP_HUD_C|GetCrosshairBorder (Variables|/Game/FirstPerson/Blueprints/BP_FirstPersonCharacter.BP_FirstPersonCharacter_C|GetHUDRef (Variables|Default|GetPlayerRef))) "Visible")
            (Audio|PlaySound2D "/Engine/VREditor/Sounds/UI/Dockable_Window_Close.Dockable_Window_Close" 1.0 1.0 0.0 0 0)
            (Pawn|Components|CharacterMovement|SetMovementMode (Variables|/Script/Engine.Character|GetCharacterMovement (Variables|Default|GetPlayerRef)) "MOVE_Walking" 0)
            (Variables|/Script/Engine.PlayerController|SetbShowMouseCursor _returnvalue_2 false)
            (Input|SetInputModeGameOnly _returnvalue_2 false)
            (Utilities|FlowControl|Delay 0.3)))
        (if (not (Variables|Default|GetdoorIsNotLocked?))
          (goto _label Reset))))))

(fn ConstructionScript)