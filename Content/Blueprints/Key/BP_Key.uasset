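; BP_Key is an interactable key pickup configured from an item data table row.
; The construction script caches the row as ItemInfo and sets its static mesh.
; Interact plays the pickup sound, then switches on a value fixed at None, so it only destroys the actor.
; The Keys branch would update the first-person character's key count and IDs and clear the crosshair before destroying it.
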(event EventBeginPlay
  (bind _asbp_first_person_character (Utilities|Casting|CastToBP_FirstPersonCharacter (Game|GetPlayerCharacter 0)))
  (Variables|Default|SetPlayerRef _asbp_first_person_character))

(event EventInteract
  (params (Character :type BP%20First%20Person%20Character%20Object%20Reference))
  (bind _playerref (Variables|Default|GetPlayerRef))
  (Development|PrintString "Interact")
  (Audio|PlaySound2D (.PickupSound (Utilities|Struct|BreakS_ItemInfo (Variables|Default|GetItemInfo))) 1.0 1.0 0.0 0 0)
  (switch Utilities|FlowControl|Switch|SwitchonE_ItemType "NewEnumerator0"
    (:NewEnumerator0
      (Actor|DestroyActor))
    (:NewEnumerator4
      (Variables|/Game/FirstPerson/Blueprints/BP_FirstPersonCharacter.BP_FirstPersonCharacter_C|SetKeysHeld _playerref (+ (Variables|/Game/FirstPerson/Blueprints/BP_FirstPersonCharacter.BP_FirstPersonCharacter_C|GetKeysHeld _playerref) 1))
      (Default|CallUpdateKeysHeld (Variables|Default|GetPlayerRef))
      (Default|CallCrosshairClear (Variables|Default|GetPlayerRef))
      (Utilities|Array|Add (Variables|/Game/FirstPerson/Blueprints/BP_FirstPersonCharacter.BP_FirstPersonCharacter_C|GetKeyID'sHeld (Variables|Default|GetPlayerRef)) (Variables|Default|GetKeyID))
      (Actor|DestroyActor))))

(fn ConstructionScript
  (bind _itemname (Variables|Default|GetItemName))
  (bind (_datatable _rowname) (Utilities|Struct|BreakDataTableRowHandle _itemname))
  (bind _returnvalue (Utilities|GetDataTableRow _datatable _rowname)
    (:then
      (bind _output_get (Variables|Default|SetItemInfo _returnvalue))
      (Components|StaticMesh|SetStaticMesh (Variables|Default|GetStaric%20Mesh) (.StaticMesh (Utilities|Struct|BreakS_ItemInfo _output_get))))))