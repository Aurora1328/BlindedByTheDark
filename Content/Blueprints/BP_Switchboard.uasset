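; Interactive switchboard actor with four clickable switches that drive two needle gauges.
; Interact hides the first-person character, disables its input, blends the view to the board and enables mouse clicks.
; Each debounced click flip-flops a switch, playing a sound and running a timeline that rotates it forward or back.
; When the timeline finishes, MoveComponentTo shifts both needles' pitch by fixed steps, accumulating across switches.
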(event OnClicked(Switch4)
  (params (TouchedComponent :type Primitive%20Component%20Object%20Reference) (ButtonPressed :type Key%20Structure :default "None"))
  (Utilities|FlowControl|DoOnce false :!label _label
    (:Completed
      (Utilities|FlowControl|Sequence
        (:then_0
          (Input|SetInputModeGameandUI (Game|GetPlayerController 0) 0 "DoNotLock" true true)
          (Utilities|FlowControl|FlipFlop
            (:A
              (Audio|PlaySound2D 0 1.0 1.0 0.0 0 0)
              (Variables|Default|SetSwitch04On true)
              (bind _value (Timeline|Timeline_1 Play)
                (:Update
                  (Transformation|SetRelativeRotation (Variables|Default|GetSwitch%204) (Math|Rotator|MakeRotator _value 0.0 0.0) false false))
                (:Finished
                  (CallFunction|Switch4))))
            (:B
              (Audio|PlaySound2D 0 1.0 1.0 0.0 0 0)
              (Variables|Default|SetSwitch04On false)
              (Timeline|Timeline_1 Reverse))))
        (:then_1
          (Utilities|FlowControl|Delay 0.3)
          (goto _label Reset))))))

(event OnClicked(Switch1)
  (params (TouchedComponent :type Primitive%20Component%20Object%20Reference) (ButtonPressed :type Key%20Structure :default "None"))
  (Utilities|FlowControl|DoOnce false :!label _label
    (:Completed
      (Utilities|FlowControl|Sequence
        (:then_0
          (Input|SetInputModeGameandUI (Game|GetPlayerController 0) 0 "DoNotLock" true true)
          (Utilities|FlowControl|FlipFlop
            (:A
              (Audio|PlaySound2D 0 1.0 1.0 0.0 0 0)
              (Variables|Default|SetSwitch01On true)
              (bind _value (Timeline|switchanimation Play)
                (:Update
                  (Transformation|SetRelativeRotation (Variables|Default|GetSwitch%201) (Math|Rotator|MakeRotator _value 0.0 0.0) false false))
                (:Finished
                  (CallFunction|Switch01))))
            (:B
              (Audio|PlaySound2D 0 1.0 1.0 0.0 0 0)
              (Variables|Default|SetSwitch01On false)
              (Timeline|switchanimation Reverse))))
        (:then_1
          (Utilities|FlowControl|Delay 0.3)
          (goto _label Reset))))))

(event OnClicked(Switch2)
  (params (TouchedComponent :type Primitive%20Component%20Object%20Reference) (ButtonPressed :type Key%20Structure :default "None"))
  (Utilities|FlowControl|DoOnce false :!label _label
    (:Completed
      (Utilities|FlowControl|Sequence
        (:then_0
          (Input|SetInputModeGameandUI (Game|GetPlayerController 0) 0 "DoNotLock" true true)
          (Utilities|FlowControl|FlipFlop
            (:A
              (Audio|PlaySound2D 0 1.0 1.0 0.0 0 0)
              (Variables|Default|SetSwitch02On true)
              (bind _value (Timeline|Timeline_0 Play)
                (:Update
                  (Transformation|SetRelativeRotation (Variables|Default|GetSwitch%202) (Math|Rotator|MakeRotator _value 0.0 0.0) false false))
                (:Finished
                  (CallFunction|Switch2))))
            (:B
              (Audio|PlaySound2D 0 1.0 1.0 0.0 0 0)
              (Variables|Default|SetSwitch02On false)
              (Timeline|Timeline_0 Reverse))))
        (:then_1
          (Utilities|FlowControl|Delay 0.3)
          (goto _label Reset))))))

(event OnClicked(Switch3)
  (params (TouchedComponent :type Primitive%20Component%20Object%20Reference) (ButtonPressed :type Key%20Structure :default "None"))
  (Utilities|FlowControl|DoOnce false :!label _label
    (:Completed
      (Utilities|FlowControl|Sequence
        (:then_0
          (Input|SetInputModeGameandUI (Game|GetPlayerController 0) 0 "DoNotLock" true true)
          (Utilities|FlowControl|FlipFlop
            (:A
              (Audio|PlaySound2D 0 1.0 1.0 0.0 0 0)
              (Variables|Default|SetSwitch03On true)
              (bind _value (Timeline|Timeline Play)
                (:Update
                  (Transformation|SetRelativeRotation (Variables|Default|GetSwitch%203) (Math|Rotator|MakeRotator _value 0.0 0.0) false false))
                (:Finished
                  (CallFunction|Switch3))))
            (:B
              (Audio|PlaySound2D 0 1.0 1.0 0.0 0 0)
              (Variables|Default|SetSwitch03On false)
              (Timeline|Timeline Reverse))))
        (:then_1
          (Utilities|FlowControl|Delay 0.3)
          (goto _label Reset))))))

(event Custom|Switch_01
  (bind _needle (Variables|Default|GetNeedle))
  (bind _needle1 (Variables|Default|GetNeedle1))
  (bind _needle_2 (Variables|Default|GetNeedle))
  (bind _needle1_2 (Variables|Default|GetNeedle1))
  (if (Variables|Default|GetSwitch01On)
    (Utilities|FlowControl|Sequence
      (:then_0
        (Components|MoveComponentTo _needle (Variables|/Script/Engine.SceneComponent|GetRelativeLocation _needle) (Math|Rotator|MakeRotator 0.0 (- (.pitch (Variables|Default|GetRelative%20Rotation)) -2e+01) 0.0) false false 0.2 false)
        (Variables|Default|SetRelative%20Rotation (Math|Rotator|MakeRotator 0.0 (- (.pitch (Variables|Default|GetRelative%20Rotation)) -2e+01) 0.0)))
      (:then_1
        (Components|MoveComponentTo _needle1 (Variables|/Script/Engine.SceneComponent|GetRelativeLocation _needle1) (Math|Rotator|MakeRotator 0.0 (- (.pitch (Variables|Default|GetRelative%20Rotation_0)) -1e+01) 0.0) false false 0.2 false)
        (Variables|Default|SetRelative%20Rotation_0 (Math|Rotator|MakeRotator 0.0 (- (.pitch (Variables|Default|GetRelative%20Rotation_0)) -1e+01) 0.0))))
    (else
      (Utilities|FlowControl|Sequence
        (:then_0
          (Components|MoveComponentTo _needle_2 (Variables|/Script/Engine.SceneComponent|GetRelativeLocation _needle_2) (Math|Rotator|MakeRotator 0.0 (- (.pitch (Variables|Default|GetRelative%20Rotation)) 2e+01) 0.0) false false 0.2 false)
          (Variables|Default|SetRelative%20Rotation (Math|Rotator|MakeRotator 0.0 (- (.pitch (Variables|Default|GetRelative%20Rotation)) 2e+01) 0.0)))
        (:then_1
          (Components|MoveComponentTo _needle1_2 (Variables|/Script/Engine.SceneComponent|GetRelativeLocation _needle1_2) (Math|Rotator|MakeRotator 0.0 (- (.pitch (Variables|Default|GetRelative%20Rotation_0)) 1e+01) 0.0) false false 0.2 false)
          (Variables|Default|SetRelative%20Rotation_0 (Math|Rotator|MakeRotator 0.0 (- (.pitch (Variables|Default|GetRelative%20Rotation_0)) 1e+01) 0.0)))))))

(event Custom|Switch4
  (bind _needle (Variables|Default|GetNeedle))
  (bind _needle1 (Variables|Default|GetNeedle1))
  (bind _needle_2 (Variables|Default|GetNeedle))
  (bind _needle1_2 (Variables|Default|GetNeedle1))
  (bind _relative_rotation_0 (Variables|Default|GetRelative%20Rotation%200))
  (bind _relative_rotation_0_2 (Variables|Default|GetRelative%20Rotation%200))
  (bind _returnvalue (- (.pitch _relative_rotation_0) 1e+01))
  (bind _returnvalue_2 (- (.pitch _relative_rotation_0_2) -1e+01))
  (if (Variables|Default|GetSwitch04On)
    (Utilities|FlowControl|Sequence
      (:then_0
        (Components|MoveComponentTo _needle_2 (Variables|/Script/Engine.SceneComponent|GetRelativeLocation _needle_2) (Math|Rotator|MakeRotator 0.0 (- (.pitch (Variables|Default|GetRelative%20Rotation)) -2e+01) 0.0) false false 0.2 false)
        (Variables|Default|SetRelative%20Rotation (Math|Rotator|MakeRotator 0.0 (- (.pitch (Variables|Default|GetRelative%20Rotation)) -2e+01) 0.0)))
      (:then_1
        (Components|MoveComponentTo _needle1_2 (Variables|/Script/Engine.SceneComponent|GetRelativeLocation _needle1_2) (Math|Rotator|MakeRotator 0.0 _returnvalue_2 0.0) false false 0.2 false)
        (Variables|Default|SetRelative%20Rotation_0 (Math|Rotator|MakeRotator 0.0 _returnvalue_2 0.0))))
    (else
      (Utilities|FlowControl|Sequence
        (:then_0
          (Components|MoveComponentTo _needle (Variables|/Script/Engine.SceneComponent|GetRelativeLocation _needle) (Math|Rotator|MakeRotator 0.0 (- (.pitch (Variables|Default|GetRelative%20Rotation)) 2e+01) 0.0) false false 0.2 false)
          (Variables|Default|SetRelative%20Rotation (Math|Rotator|MakeRotator 0.0 (- (.pitch (Variables|Default|GetRelative%20Rotation)) 2e+01) 0.0)))
        (:then_1
          (Components|MoveComponentTo _needle1 (Variables|/Script/Engine.SceneComponent|GetRelativeLocation _needle1) (Math|Rotator|MakeRotator 0.0 _returnvalue 0.0) false false 0.2 false)
          (Variables|Default|SetRelative%20Rotation_0 (Math|Rotator|MakeRotator 0.0 _returnvalue 0.0)))))))

(event Custom|Switch2
  (bind _needle (Variables|Default|GetNeedle))
  (bind _needle1 (Variables|Default|GetNeedle1))
  (bind _needle_2 (Variables|Default|GetNeedle))
  (bind _needle1_2 (Variables|Default|GetNeedle1))
  (bind _relative_rotation_0 (Variables|Default|GetRelative%20Rotation%200))
  (bind _relative_rotation_0_2 (Variables|Default|GetRelative%20Rotation%200))
  (bind _returnvalue (- (.pitch _relative_rotation_0_2) -1e+01))
  (bind _returnvalue_2 (- (.pitch _relative_rotation_0) 1e+01))
  (if (Variables|Default|GetSwitch02On)
    (Utilities|FlowControl|Sequence
      (:then_0
        (Components|MoveComponentTo _needle (Variables|/Script/Engine.SceneComponent|GetRelativeLocation _needle) (Math|Rotator|MakeRotator 0.0 (- (.pitch (Variables|Default|GetRelative%20Rotation)) -2e+01) 0.0) false false 0.2 false)
        (Variables|Default|SetRelative%20Rotation (Math|Rotator|MakeRotator 0.0 (- (.pitch (Variables|Default|GetRelative%20Rotation)) -2e+01) 0.0)))
      (:then_1
        (Components|MoveComponentTo _needle1 (Variables|/Script/Engine.SceneComponent|GetRelativeLocation _needle1) (Math|Rotator|MakeRotator 0.0 _returnvalue 0.0) false false 0.2 false)
        (Variables|Default|SetRelative%20Rotation_0 (Math|Rotator|MakeRotator 0.0 _returnvalue 0.0))))
    (else
      (Utilities|FlowControl|Sequence
        (:then_0
          (Components|MoveComponentTo _needle_2 (Variables|/Script/Engine.SceneComponent|GetRelativeLocation _needle_2) (Math|Rotator|MakeRotator 0.0 (- (.pitch (Variables|Default|GetRelative%20Rotation)) 2e+01) 0.0) false false 0.2 false)
          (Variables|Default|SetRelative%20Rotation (Math|Rotator|MakeRotator 0.0 (- (.pitch (Variables|Default|GetRelative%20Rotation)) 2e+01) 0.0)))
        (:then_1
          (Components|MoveComponentTo _needle1_2 (Variables|/Script/Engine.SceneComponent|GetRelativeLocation _needle1_2) (Math|Rotator|MakeRotator 0.0 _returnvalue_2 0.0) false false 0.2 false)
          (Variables|Default|SetRelative%20Rotation_0 (Math|Rotator|MakeRotator 0.0 _returnvalue_2 0.0)))))))

(event Custom|Switch3
  (bind _needle (Variables|Default|GetNeedle))
  (bind _needle1 (Variables|Default|GetNeedle1))
  (bind _needle_2 (Variables|Default|GetNeedle))
  (bind _needle1_2 (Variables|Default|GetNeedle1))
  (bind _relative_rotation_0 (Variables|Default|GetRelative%20Rotation%200))
  (bind _relative_rotation_0_2 (Variables|Default|GetRelative%20Rotation%200))
  (bind _returnvalue (- (.pitch _relative_rotation_0_2) -1e+01))
  (bind _returnvalue_2 (- (.pitch _relative_rotation_0) 1e+01))
  (if (Variables|Default|GetSwitch03On)
    (Utilities|FlowControl|Sequence
      (:then_0
        (Components|MoveComponentTo _needle (Variables|/Script/Engine.SceneComponent|GetRelativeLocation _needle) (Math|Rotator|MakeRotator 0.0 (- (.pitch (Variables|Default|GetRelative%20Rotation)) -2e+01) 0.0) false false 0.2 false)
        (Variables|Default|SetRelative%20Rotation (Math|Rotator|MakeRotator 0.0 (- (.pitch (Variables|Default|GetRelative%20Rotation)) -2e+01) 0.0)))
      (:then_1
        (Components|MoveComponentTo _needle1 (Variables|/Script/Engine.SceneComponent|GetRelativeLocation _needle1) (Math|Rotator|MakeRotator 0.0 _returnvalue 0.0) false false 0.2 false)
        (Variables|Default|SetRelative%20Rotation_0 (Math|Rotator|MakeRotator 0.0 _returnvalue 0.0))))
    (else
      (Utilities|FlowControl|Sequence
        (:then_0
          (Components|MoveComponentTo _needle_2 (Variables|/Script/Engine.SceneComponent|GetRelativeLocation _needle_2) (Math|Rotator|MakeRotator 0.0 (- (.pitch (Variables|Default|GetRelative%20Rotation)) 2e+01) 0.0) false false 0.2 false)
          (Variables|Default|SetRelative%20Rotation (Math|Rotator|MakeRotator 0.0 (- (.pitch (Variables|Default|GetRelative%20Rotation)) 2e+01) 0.0)))
        (:then_1
          (Components|MoveComponentTo _needle1_2 (Variables|/Script/Engine.SceneComponent|GetRelativeLocation _needle1_2) (Math|Rotator|MakeRotator 0.0 _returnvalue_2 0.0) false false 0.2 false)
          (Variables|Default|SetRelative%20Rotation_0 (Math|Rotator|MakeRotator 0.0 _returnvalue_2 0.0)))))))

(event Collision|EventActorBeginOverlap
  (params (OtherActor :type Actor%20Object%20Reference)))

(event EventTick
  (params (DeltaSeconds :type Float%20%28single-precision%29)))

(event EventInteract
  (params (Character :type BP%20First%20Person%20Character%20Object%20Reference))
  (bind _returnvalue (Game|GetPlayerController 0))
  (Class|WidgetBlueprintLibrary|SetFocustoGameViewport)
  (Utilities|FlowControl|DoOnce false :!label _label
    (:Completed
      (Utilities|FlowControl|Sequence
        (:then_0
          (bind _asbp_first_person_character (Utilities|Casting|CastToBP_FirstPersonCharacter (Game|GetPlayerCharacter 0)))
          (Rendering|SetActorHiddenInGame _asbp_first_person_character true)
          (Input|DisableInput _asbp_first_person_character _returnvalue)
          (Game|Player|SetViewTargetwithBlend _returnvalue self 0.5 "VTBlend_Linear" 0.0 false)
          (Variables|/Script/Engine.PlayerController|SetbShowMouseCursor _returnvalue true)
          (Variables|/Script/Engine.PlayerController|SetbEnableClickEvents _returnvalue true))
        (:then_1
          (Utilities|FlowControl|Delay 1.0)
          (goto _label Reset))))))

(event EventBeginPlay
  (Variables|Default|SetRelative%20Rotation (Variables|/Script/Engine.SceneComponent|GetRelativeRotation (Variables|Default|GetNeedle)))
  (Variables|Default|SetRelative%20Rotation_0 (Variables|/Script/Engine.SceneComponent|GetRelativeRotation (Variables|Default|GetNeedle1))))

(fn ConstructionScript)